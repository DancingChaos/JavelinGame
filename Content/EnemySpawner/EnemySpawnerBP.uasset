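; Enemy spawner Blueprint that repeatedly creates EnemyBP actors at random heights.
; Tick drives a Delay, which ignores re-triggers while counting down, so it acts as a repeating timer set by SpawnDelay.
; Each spawn takes X, Y, rotation and scale from the Arrow component, with Z randomized between the TopBorder and BotBorder variables.
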(event `self.ReceiveTick`
  (params (DeltaSeconds :type "Float (single-precision)"))
  (`KismetSystemLibrary.Delay` (`self.SpawnDelay`))
  (`|SpawnActorFromClass` "/Game/Enemy/EnemyBP.EnemyBP_C" (`KismetMathLibrary.MakeTransform` (`KismetMathLibrary.MakeVector` (.x (.location (`SceneComponent.K2_GetComponentToWorld` (`self.Arrow`)))) (.y (.location (`SceneComponent.K2_GetComponentToWorld` (`self.Arrow`)))) (`KismetMathLibrary.RandomFloatInRange` (`self.TopBorder`) (`self.BotBorder`))) (.rotation (`SceneComponent.K2_GetComponentToWorld` (`self.Arrow`))) (.scale (`SceneComponent.K2_GetComponentToWorld` (`self.Arrow`)))) "Undefined" "OverrideRootScale" null null))

(fn `UserConstructionScript`)