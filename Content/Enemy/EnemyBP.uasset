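; Enemy actor with a flipbook sprite and projectile movement that dies on contact with either a BirdBP or the 2D side-scroller player character.
; A bird overlap destroys the bird and later grants the player a kill reward, while a player overlap deals damage with no reward.
; Both paths set a death flag, play death flipbook and hit sound, halt movement, then destroy the enemy after a short delay.
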(event `self.BoxCollision.OnComponentBeginOverlap`
  (params (OverlappedComponent :type "PrimitiveComponent Object Reference") (OtherActor :type "Actor Object Reference") (OtherComp :type "PrimitiveComponent Object Reference") (OtherBodyIndex :type Integer) (bFromSweep :type Boolean) (SweepResult :type "HitResult Structure (by ref)"))
  (bind _returnvalue (`GameplayStatics.GetObjectClass` OtherActor))
  (if (and (not (`self.IsDead`)) (== _returnvalue "/Game/Character/Items/BirdProjectile/BirdBP.BirdBP_C"))
    (`self.K2_DestroyActor` OtherActor)
    (set `self.IsDead` true)
    (`/Engine/EditorBlueprintResources/StandardMacros.DoOnce` false
      (:`Completed`
        (`|ExecutionSequence`
          (:`then_0`
            (`PaperFlipbookComponent.SetFlipbook` (`self.PaperFlipbook`) "/Game/Enemy/Flipbooks/Death.Death")
            (`GameplayStatics.PlaySound2D` "/Game/Resources/Music/Hit.Hit" 0.01 1.0 0.0 null null false))
          (:`then_1`
            (`ProjectileMovementComponent.SetVelocityInLocalSpace` (`self.ProjectileMovement`) (0.0 0.0 0.0))
            (set `ProjectileMovementComponent.InitialSpeed` 0.0 (`self.ProjectileMovement`)))
          (:`then_2`
            (`KismetSystemLibrary.Delay` 0.5)
            (bind _as2dside_scroller_character (cast `/Game/Character/2DSideScrollerCharacter` (`GameplayStatics.GetPlayerCharacter` 0)))
            (`/Game/Character/2DSideScrollerCharacter.AddKillReward` _as2dside_scroller_character)
            (`self.K2_DestroyActor`)))))
    (elif (and (== _returnvalue "/Game/Character/2DSideScrollerCharacter.2DSideScrollerCharacter_C") (not (`self.IsDead`)))
      (set `self.IsDead` true)
      (bind _as2dside_scroller_character_2 (cast `/Game/Character/2DSideScrollerCharacter` (`GameplayStatics.GetPlayerCharacter` 0)))
      (`/Game/Character/2DSideScrollerCharacter.Get Damage by Enemy` _as2dside_scroller_character_2 (`self.Damage`))
      (`/Engine/EditorBlueprintResources/StandardMacros.DoOnce` false
        (:`Completed`
          (`|ExecutionSequence`
            (:`then_0`
              (`PaperFlipbookComponent.SetFlipbook` (`self.PaperFlipbook`) "/Game/Enemy/Flipbooks/Death.Death")
              (`GameplayStatics.PlaySound2D` "/Game/Resources/Music/Hit.Hit" 0.01 1.0 0.0 null null false))
            (:`then_1`
              (`ProjectileMovementComponent.SetVelocityInLocalSpace` (`self.ProjectileMovement`) (0.0 0.0 0.0))
              (set `ProjectileMovementComponent.InitialSpeed` 0.0 (`self.ProjectileMovement`)))
            (:`then_2`
              (`KismetSystemLibrary.Delay` 0.5)
              (`self.K2_DestroyActor`))))))))

(fn `UserConstructionScript`)